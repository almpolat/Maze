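; Modular maze cell that procedurally builds its geometry and runs a game countdown.
; The Construction Script sizes the floor, optional walls and ceiling from grid settings, adding a point light that is either green or gates optional box colliders.
; Tick decrements GameTime, pausing at 101 or above; at zero it reddens the light, flags a loss, pauses and queues a delayed NewMap load.
; The west-box overlap only casts to the character.
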(event `self.ReceiveTick`
  (params (DeltaSeconds :type "Float (single-precision)"))
  (bind _gametime (`self.GameTime`))
  (if (>= _gametime 101.0)
    (`GameplayStatics.SetGamePaused` true)
    (else
      (bind _output_get (set `self.GameTime` (- _gametime DeltaSeconds)))
      (if (<= _output_get 0.0)
        (bind _output_get_2 (set `self.New Light Color` (struct :`R` 0.463542 :`B` 0.03063 :`A` 1.0)))
        (`LightComponent.SetLightColor` (`self.LightComp`) _output_get_2 true)
        (set `self.GameLose` true)
        (`GameplayStatics.SetGamePaused` true)
        (`KismetSystemLibrary.Delay` 2.0)
        (`GameplayStatics.OpenLevel` "NewMap")))))

(event `self.WestBoxColl.OnComponentBeginOverlap`
  (params (OverlappedComponent :type "PrimitiveComponent Object Reference") (OtherActor :type "Actor Object Reference") (OtherComp :type "PrimitiveComponent Object Reference") (OtherBodyIndex :type Integer) (bFromSweep :type Boolean) (SweepResult :type "HitResult Structure (by ref)"))
  (cast `/Game/Labs/Lab1/BP_ThirdPersonCharacter` OtherActor))

(fn `UserConstructionScript`
  (locals (walllenght :type "Float (double-precision)") (wallthickness :type "Float (double-precision)"))
  (bind _walllenght (`local.walllenght`))
  (bind _gridsize (`self.gridsize`))
  (bind _returnvalue (* (`local.walllenght`) 0.5))
  (bind _returnvalue_2 (* (`local.walllenght`) 0.5))
  (set `local.walllenght` _gridsize)
  (set `local.wallthickness` (* _gridsize 0.1))
  (`SceneComponent.SetRelativeScale3D` (`self.floor`) (`self.NewMacro` (`KismetMathLibrary.MakeVector` _walllenght _walllenght (`local.wallthickness`))))
  (if (`self.WestWall`)
    (`AddComponent|NODE_AddStaticMeshComponent-0` :`RelativeTransform` (`KismetMathLibrary.MakeTransform` (0.0 0.0 0.0) (struct) (`self.NewMacro` (`KismetMathLibrary.MakeVector` (`local.walllenght`) (`local.wallthickness`) (`self.wallheight`))))))
  (if (`self.SouthWal`)
    (`AddComponent|NODE_AddStaticMeshComponent-1` :`RelativeTransform` (`KismetMathLibrary.MakeTransform` (0.0 0.0 0.0) (struct) (`self.NewMacro` (`KismetMathLibrary.MakeVector` (`local.wallthickness`) (`local.walllenght`) (`self.wallheight`))))))
  (if (`self.EastWall`)
    (`AddComponent|NODE_AddStaticMeshComponent-2` :`RelativeTransform` (`KismetMathLibrary.MakeTransform` (`KismetMathLibrary.MakeVector` 0.0 (- (`local.walllenght`) (`local.wallthickness`))) (struct) (`self.NewMacro` (`KismetMathLibrary.MakeVector` (`local.walllenght`) (`local.wallthickness`) (`self.wallheight`))))))
  (if (`self.NorthWall`)
    (`AddComponent|NODE_AddStaticMeshComponent-3` :`RelativeTransform` (`KismetMathLibrary.MakeTransform` (`KismetMathLibrary.MakeVector` (- (`local.walllenght`) (`local.wallthickness`))) (struct) (`self.NewMacro` (`KismetMathLibrary.MakeVector` (`local.wallthickness`) (`local.walllenght`) (`self.wallheight`))))))
  (if (`self.cell`)
    (`AddComponent|NODE_AddStaticMeshComponent-4` :`RelativeTransform` (`KismetMathLibrary.MakeTransform` (`KismetMathLibrary.MakeVector` 0.0 0.0 (`self.wallheight`)) (struct) (`self.NewMacro` (`KismetMathLibrary.MakeVector` (`self.wallheight`) (`local.walllenght`) (`local.wallthickness`))))))
  (if (> (`self.light`) 0.0)
    (bind _returnvalue_3 (`AddComponent|NODE_AddPointLightComponent-0` :`RelativeTransform` (`KismetMathLibrary.MakeTransform` (`KismetMathLibrary.MakeVector` _returnvalue _returnvalue (- (`self.wallheight`) (`local.wallthickness`))))))
    (bind _output_get (set `self.LightComp` _returnvalue_3))
    (`LightComponent.SetIntensity` _output_get (`self.light`))
    (if (`self.ChangeLightGreen`)
      (`ActorComponent.K2_DestroyComponent` _output_get)
      (bind _returnvalue_4 (`AddComponent|NODE_AddPointLightComponent-1` :`RelativeTransform` (`KismetMathLibrary.MakeTransform` (`KismetMathLibrary.MakeVector` _returnvalue_2 _returnvalue_2 (- (`self.wallheight`) (`local.wallthickness`))))))
      (`LightComponent.SetLightColor` _returnvalue_4 (struct :`G` 1.0 :`B` 0.123422 :`A` 1.0) true)
      (else
        (`LightComponent.SetLightColor` _output_get (`self.New Light Color`) true)
        (if (`self.SouthBox`)
          (`AddComponent|NODE_AddBoxComponent-2` :`RelativeTransform` (`KismetMathLibrary.MakeTransform` (0.0 250.0 100.0) (struct) (`self.NewMacro` (`KismetMathLibrary.MakeVector` (`local.wallthickness`) (`local.walllenght`) (`self.wallheight`))))))
        (if (`self.EastBox`)
          (`AddComponent|NODE_AddBoxComponent-3` :`RelativeTransform` (`KismetMathLibrary.MakeTransform` (`KismetMathLibrary.MakeVector` 250.0 (- (`local.walllenght`) (`local.wallthickness`)) 100.0) (struct) (`self.NewMacro` (`KismetMathLibrary.MakeVector` (`local.walllenght`) (`local.wallthickness`) (`self.wallheight`))))))
        (if (`self.NorthBox`)
          (`AddComponent|NODE_AddBoxComponent-1` :`RelativeTransform` (`KismetMathLibrary.MakeTransform` (`KismetMathLibrary.MakeVector` (- (`local.walllenght`) (`local.wallthickness`)) 250.0 100.0) (struct) (`self.NewMacro` (`KismetMathLibrary.MakeVector` (`local.wallthickness`) (`local.walllenght`) (`self.wallheight`))))))
        (if (`self.WestBox`)
          (bind _returnvalue_5 (`AddComponent|NODE_AddBoxComponent-4` :`RelativeTransform` (`KismetMathLibrary.MakeTransform` (250.0 0.0 100.0) (struct) (`self.NewMacro` (`KismetMathLibrary.MakeVector` (`local.walllenght`) (`local.wallthickness`) (`self.wallheight`))))))
          (set `self.WestBoxColl` _returnvalue_5))))))